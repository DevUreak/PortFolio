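; AI_Nexus_BP is a Nexus actor Blueprint that drives its MonsterHP health bar widget.
; On BeginPlay it casts the widget to Monster_HUD and sets a fixed maximum health.
; The RefreshHPBar2 event converts the supplied health to an integer, passes it to the HUD's DelayRefreshHP and prints debug messages.
; No damage or AI logic appears in these graphs.
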(event `self.ReceiveBeginPlay`
  (bind _asmonster_hud (cast `/Game/GameSystem/BluePrint/Monster_HUD` (`WidgetComponent.GetUserWidgetObject` (`self.MonsterHP`))))
  (set `/Game/GameSystem/BluePrint/Monster_HUD.MonsterMaxHelath` 400 _asmonster_hud))

(event `RefreshHPBar2`
  (params (nowHealth :type String))
  (bind _returnvalue (`KismetStringLibrary.Conv_StringToInt` nowHealth))
  (bind _asmonster_hud (cast `/Game/GameSystem/BluePrint/Monster_HUD` (`WidgetComponent.GetUserWidgetObject` (`self.MonsterHP`))))
  (`/Game/GameSystem/BluePrint/Monster_HUD.DelayRefreshHP` _asmonster_hud _returnvalue)
  (`KismetSystemLibrary.PrintString` "hp change!")
  (`KismetSystemLibrary.PrintString` (`KismetStringLibrary.Conv_IntToString` _returnvalue)))

(fn `UserConstructionScript`)