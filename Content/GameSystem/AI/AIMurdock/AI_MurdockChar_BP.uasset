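; Murdock AI monster character Blueprint that drives its overhead HP bar and exposes movement, attack and death state flags.
; InitMonsterRef finds its monster object by index in the game instance's spawn list; Tick copies its attacking/alive values and flags zero velocity as stopped.
; Tick also rotates the widget using the main camera's rotation with fixed pitch, while events set up and refresh Monster_HUD health.
; StopAttacking clears the attacking flag, and DeathDestroyBP triggers final destruction.
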(event `self.ReceiveBeginPlay`
  ;[1 1 1] HP BAR HUB ROATION STATIC
  (bind _outactors (`GameplayStatics.GetAllActorsOfClass` "/Script/AgeofWarGameClient2.MainCamerra"))
  (for _array_element _outactors
    (set `self.MainCamera` _array_element)))

(event `self.ReceiveTick`
  (params (DeltaSeconds :type "Float (single-precision)"))
  (bind _monsterbasebp (`self.MonsterBaseBP`))
  ;[1 1 1] HP BAR HUB ROATION STATIC
  (`SceneComponent.K2_SetWorldRotation` (`self.Widget`) (`KismetMathLibrary.MakeRotator` (.roll (`KismetMathLibrary.FindLookAtRotation` (`KismetMathLibrary.Conv_RotatorToVector` (`SceneComponent.K2_GetComponentRotation` (`self.Widget`))) (`KismetMathLibrary.Conv_RotatorToVector` (`SceneComponent.K2_GetComponentRotation` (`Actor.RootComponent` (`self.MainCamera`)))))) 70.0 (.yaw (`KismetMathLibrary.FindLookAtRotation` (`KismetMathLibrary.Conv_RotatorToVector` (`SceneComponent.K2_GetComponentRotation` (`self.Widget`))) (`KismetMathLibrary.Conv_RotatorToVector` (`SceneComponent.K2_GetComponentRotation` (`Actor.RootComponent` (`self.MainCamera`))))))) false false)
  (if (== 0.0 (`KismetMathLibrary.VSize` (`MovementComponent.Velocity` (`self.CharacterMovement`))))
    (set `self.MoveFlag` true)
    (else
      (set `self.MoveFlag` false)))
  ;[1 1 1] attacking task에서 수정한 attaking 값을 계속 읽어옴
  (`/Engine/EditorBlueprintResources/StandardMacros.IsValid` _monsterbasebp
    (:`Is Valid`
      (set `self.MurdockATTACKINGFlagBP` (`MonsterBase.MonsterATTAKING` _monsterbasebp))
      (set `self.MurdockDeathFlagBP` (`MonsterBase.MonsterAlive` _monsterbasebp)))))

(event `ChangeHPBar`
  (params (intFarm :type String) (MAXHealath :type String))
  (bind _asaowgame_instance (cast `AOWGameInstance` (`GameplayStatics.GetGameInstance`)))
  (bind _output_get (set `self.GameInstacne` _asaowgame_instance)) ; 인스턴스 초기화
  (bind _asmonster_hud (cast `/Game/GameSystem/BluePrint/Monster_HUD` (`WidgetComponent.GetUserWidgetObject` (`self.Widget`))))
  (`/Game/GameSystem/BluePrint/Monster_HUD.HPChangeColor` _asmonster_hud (`KismetStringLibrary.Conv_StringToInt` intFarm) (`.userType` (break `CustomStructGameOption` (`AOWGameInstance.fsGameOption` _output_get))) (`KismetStringLibrary.Conv_StringToInt` MAXHealath)))

(event `InitMonsterRef`
  (params (MonsterIndex :type String))
  (bind _returnvalue (`KismetStringLibrary.Conv_StringToInt` MonsterIndex))
  (bind _asaowgame_instance (cast `AOWGameInstance` (`GameplayStatics.GetGameInstance`)))
  (set `self.MonsterIndexBP` _returnvalue)
  (for _array_element (`AOWGameInstance.SpawnMonsterList` _asaowgame_instance) :!label _label
    (if (== _returnvalue (`MonsterBase.monsterIndex` _array_element))
      (`self.breakloop`)
      (set `self.MonsterBaseBP` _array_element))))

(event `breakloop`
  (goto _label :!via `Break`))

(event `RefreshHPBar`
  (params (nowHealth :type String))
  (bind _asmonster_hud (cast `/Game/GameSystem/BluePrint/Monster_HUD` (`WidgetComponent.GetUserWidgetObject` (`self.Widget`))))
  (`/Game/GameSystem/BluePrint/Monster_HUD.DelayRefreshHP` _asmonster_hud (`KismetStringLibrary.Conv_StringToInt` nowHealth)))

(event `DeathDestroyBP`
  (`self.MonsterDeathDestoryFinal`)
  (`KismetSystemLibrary.PrintString` "Death Final"))

(fn `StopAttacking`
  (set `MonsterBase.MonsterATTAKING` false (`self.MonsterBaseBP`)))

(fn `UserConstructionScript`)